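; First-person player character Blueprint handling a camera FOV effect, footstep and pickup audio, and highlighting of looked-at objects.
; E runs three chained FOV timelines, locked until the last finishes, while a cooldown timeline plays footsteps during acceleration.
; Interactor events trigger the pickup sound and toggle custom depth on the looked-at actor's first tagged primitive for outlining.
; A deprecated dissolve timeline driving a material parameter collection remains disconnected.
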(event `Key|One`
  (params (Key :type "Key Structure"))
  ;[1 1 1] Dissolve Timeline (DEPRECATED)
)

(event `Key|E`
  (params (Key :type "Key Structure"))
  ;[1 1 1] FoV timeline
  (:`Pressed`
    (if (`self.Allowance`)
      (set `self.Allowance` false)
      (bind (_direction _newtrack_0) (`Timeline|Increase FOV` :!via `PlayFromStart`)
        (:`Update`
          (`CameraComponent.SetFieldOfView` (`self.FirstPersonCameraComponent`) _newtrack_0))
        (:`Finished`
          (bind (_direction_2 _newtrack_0_2) (`Timeline|Lower FOV` :!via `PlayFromStart`)
            (:`Update`
              (`CameraComponent.SetFieldOfView` (`self.FirstPersonCameraComponent`) _newtrack_0_2))
            (:`Finished`
              (bind (_direction_3 _newtrack_0_3) (`Timeline|Reset FOV` :!via `PlayFromStart`)
                (:`Update`
                  (`CameraComponent.SetFieldOfView` (`self.FirstPersonCameraComponent`) _newtrack_0_3))
                (:`Finished`
                  (set `self.Allowance` true))))))))))

(event `self.ReceiveTick`
  (params (DeltaSeconds :type "Float (single-precision)"))
  ;[1 1 1] Very hacky footsteps
  (if (!= (`CharacterMovementComponent.GetCurrentAcceleration` (`self.CharacterMovement`)) (0.0 0.0 0.0))
    (`Timeline|AudioCooldown` :!label _label
      (:`Finished`
        (`GameplayStatics.PlaySound2D` "/Game/Audio/footstep.footstep")
        (goto _label :!via `SetNewTime`)))
    (else
      (goto _label :!via `Stop`))))

(event `self.Interactor.on_pickup`
  (`GameplayStatics.PlaySound2D` "/Game/Audio/pickup.pickup"))

(event `self.Interactor.trace_hit`
  (params (trace :type Boolean))
  ;[1 1 1] Highlight objects when looking at them
  (if trace
    (`self.StartRenderOutline` (`self.Actor`))
    (else
      (`/Engine/EditorBlueprintResources/StandardMacros.DoOnce` true :!label _label_2
        (:`Completed`
          (`self.StopRenderOutline` (`self.Actor`)))))))

(event `self.Interactor.looking_at_object`
  (params (actor :type "Actor Object Reference"))
  ;[1 1 1] Highlight objects when looking at them
  (set `self.Actor` actor)
  (goto _label_2 :!via `Reset`))

(fn `StartRenderOutline`
  (params (Actor :type "Actor Object Reference"))
  (`PrimitiveComponent.SetRenderCustomDepth` (`|GetArrayItem` (`self.GetComponentsByTag` Actor "/Script/Engine.PrimitiveComponent" (`self.Tag`))) true))

(fn `StopRenderOutline`
  (params (Actor :type "Actor Object Reference"))
  (`PrimitiveComponent.SetRenderCustomDepth` (`|GetArrayItem` (`self.GetComponentsByTag` Actor "/Script/Engine.PrimitiveComponent" (`self.Tag`))) false))

(fn `UserConstructionScript`)