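; Interactable button that slides its linked actor, apparently a bookshelf, along the world X axis.
; It caches the linked actor's location at BeginPlay, and an InteractComponent request plays a timeline that offsets the actor from that position.
; The timeline only starts while the actor sits at its initial location; otherwise the button prints that the target cannot move further right.
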(event `self.ReceiveBeginPlay`
  (bind _returnvalue (`self.GetLinkedActor`))
  (set `self.LinkedInitialLocation` (`self.K2_GetActorLocation` _returnvalue)))

(event `self.InteractComponent.OnInteractRequest`
  (bind _returnvalue (`self.GetLinkedActor`))
  (if (== (`self.K2_GetActorLocation` _returnvalue) (`self.LinkedInitialLocation`) :`ErrorTolerance` 0.0003)
    (bind (_direction _bookshelfanimation) (`Timeline|Timeline_0` :!via `PlayFromStart`)
      (:`Update`
        (bind _returnvalue_2 (`self.GetLinkedActor`))
        (`self.K2_SetActorLocation` _returnvalue_2 (+ (`KismetMathLibrary.MakeVector` _bookshelfanimation) (`self.LinkedInitialLocation`)) false false)))
    (else
      (`KismetSystemLibrary.PrintText` "Cannot move target more right." true false))))

(fn `UserConstructionScript`
  (`parent.UserConstructionScript`))