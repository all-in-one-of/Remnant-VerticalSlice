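; Mirror controller that repositions its owning actor relative to the first player character every frame.
; Each Tick places the owner 200 units along the player's forward vector, in front of the character.
; The VInterpTo has no interp speed set, so it snaps to the target rather than easing.
; The look-at rotation uses the player location as both start and target, so it yields no meaningful facing.
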(event `self.ReceiveTick`
  (params (DeltaSeconds :type "Float (single-precision)"))
  (bind _returnvalue (`GameplayStatics.GetPlayerCharacter` 0))
  (bind _returnvalue_2 (`GameplayStatics.GetPlayerCharacter` 0))
  (bind _returnvalue_3 (`Actor.K2_GetActorLocation` _returnvalue))
  (`Actor.K2_SetActorLocationAndRotation` (`self.GetOwner`) (`KismetMathLibrary.VInterpTo` (`Actor.K2_GetActorLocation` _returnvalue_2) (+ (* (* (`Actor.GetActorForwardVector` _returnvalue) -1) -200.0) _returnvalue_3) DeltaSeconds) (`KismetMathLibrary.FindLookAtRotation` (`Actor.K2_GetActorLocation` _returnvalue_2) _returnvalue_3) false false))