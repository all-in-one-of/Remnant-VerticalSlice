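; LeverRight_BP is a puzzle lever that signals the bookshelf cannot move further right when the player interacts with it.
; It stores its starting rotation on BeginPlay.
; An interact request prints that message and plays a timeline whose BrokenLever track drives pitch, combined with the start rotation, to animate the lever without moving anything else.
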(event `self.ReceiveBeginPlay`
  (set `self.StartRotation` (`self.K2_GetActorRotation`)))

(event `self.InteractComponent.OnInteractRequest`
  (`KismetSystemLibrary.PrintText` "Cannot move the bookshelf more right" true false)
  (bind (_direction _broken_lever) (`Timeline|Timeline_0` :!via `PlayFromStart`)
    (:`Update`
      (`self.K2_SetActorRotation` (`KismetMathLibrary.ComposeRotators` (`KismetMathLibrary.MakeRotator` 0.0 _broken_lever) (`self.StartRotation`))))))

(fn `UserConstructionScript`
  (`parent.UserConstructionScript`))