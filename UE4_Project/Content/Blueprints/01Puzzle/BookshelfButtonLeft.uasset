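; Puzzle button for the left side of a bookshelf puzzle, which needs a lever fitted before it works.
; On the first interaction, it checks the player pawn's inventory component for "LeftLever" and, if present, sets LeverPlaced and toggles the lever mesh's visibility.
; Once the lever is placed, each interaction calls MoveLeft on the linked Puzzle01_Bookshelf_BP actor.
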(event `self.ReceiveBeginPlay`
  (set `self.LeverPlaced` false))

(event `self.InteractComponent.OnInteractRequest`
  (if (`self.LeverPlaced`)
    (bind _returnvalue (`self.GetLinkedActor`))
    (bind _aspuzzle_01_bookshelf_bp (cast `/Game/Blueprints/01Puzzle/Puzzle01_Bookshelf_BP` _returnvalue))
    (`Puzzle01_Bookshelf.MoveLeft` _aspuzzle_01_bookshelf_bp)
    (else
      (bind _asplayer_fpp_bp (cast `/Game/Blueprints/PlayerFPP_BP` (`GameplayStatics.GetPlayerPawn` 0)))
      (if (`InventoryComponent.HasItem` (`self.GetComponentByClass` _asplayer_fpp_bp "/Script/TimeyWimey.InventoryComponent") "LeftLever")
        (set `self.LeverPlaced` true)
        (`SceneComponent.ToggleVisibility` (`self.LeverMesh`) false)))))

(fn `UserConstructionScript`
  (`parent.UserConstructionScript`))