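; MachineKeyInteractable_BP is a puzzle key receptacle that starts two linked machines when the player interacts while holding the MachineKey.
; On an interact request, it checks the player's InventoryComponent for the item without removing it.
; On success, it toggles the key mesh's visibility, sets KeyPlaced to block repeat use, then calls StartMachine on both linked Puzzle01_Machine actors in sequence.
; A failed cast on the first machine also prevents the second from starting.
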(event `self.ReceiveBeginPlay`
  (set `self.KeyPlaced` false))

(event `self.InteractComponent.OnInteractRequest`
  (if (not (`self.KeyPlaced`))
    (bind _asplayer_fpp_bp (cast `/Game/Blueprints/PlayerFPP_BP` (`GameplayStatics.GetPlayerPawn` 0)))
    (if (`InventoryComponent.HasItem` (`self.GetComponentByClass` _asplayer_fpp_bp "/Script/TimeyWimey.InventoryComponent") "MachineKey")
      (`SceneComponent.ToggleVisibility` (`self.KeyMesh`) false)
      (set `self.KeyPlaced` true)
      (bind _returnvalue (`self.GetLinkedActorOne`))
      (bind _aspuzzle_01_machine (cast `Puzzle01_Machine` _returnvalue))
      (`Puzzle01_Machine.StartMachine` _aspuzzle_01_machine)
      (bind _returnvalue_2 (`self.GetLinkedActorTwo`))
      (bind _aspuzzle_01_machine_2 (cast `Puzzle01_Machine` _returnvalue_2))
      (`Puzzle01_Machine.StartMachine` _aspuzzle_01_machine_2))))

(fn `UserConstructionScript`
  (`parent.UserConstructionScript`))