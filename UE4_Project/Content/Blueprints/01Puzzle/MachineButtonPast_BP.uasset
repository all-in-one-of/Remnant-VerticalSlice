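; Past-era machine button for Puzzle 01, an interactable socket where the player places a button that then drives the moving bookshelves.
; The first interaction checks the player's inventory for the MachineButton item, then toggles its own mesh visibility and marks the button placed.
; Placing it also toggles the linked present-era button's mesh and enables that actor.
; Later interactions call SwitchSequence on the second linked actor, the bookshelves.
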(event `self.ReceiveBeginPlay`
  (set `self.ButtonPlaced` false))

(event `self.InteractComponent.OnInteractRequest`
  (if (`self.ButtonPlaced`)
    (bind _returnvalue (`self.GetLinkedActorTwo`))
    (bind _aspuzzle_01_moving_bookshelves (cast `Puzzle01_MovingBookshelves` _returnvalue))
    (`Puzzle01_MovingBookshelves.SwitchSequence` _aspuzzle_01_moving_bookshelves)
    (else
      (bind _asplayer_fpp_bp (cast `/Game/Blueprints/PlayerFPP_BP` (`GameplayStatics.GetPlayerPawn` 0)))
      (if (`InventoryComponent.HasItem` (`self.GetComponentByClass` _asplayer_fpp_bp "/Script/TimeyWimey.InventoryComponent") "MachineButton")
        (`SceneComponent.ToggleVisibility` (`self.Mesh`) false)
        (set `self.ButtonPlaced` true)
        (bind _returnvalue_2 (`self.GetLinkedActorOne`))
        (bind _asmachine_button_present_bp (cast `/Game/Blueprints/01Puzzle/MachineButtonPresent_BP` _returnvalue_2))
        (`SceneComponent.ToggleVisibility` (`/Game/Blueprints/01Puzzle/MachineButtonPresent_BP.Mesh` _asmachine_button_present_bp) false)
        (set `/Game/Blueprints/01Puzzle/MachineButtonPresent_BP.Enabled` true _asmachine_button_present_bp)))))

(fn `UserConstructionScript`
  (`parent.UserConstructionScript`))