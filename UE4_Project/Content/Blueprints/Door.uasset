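; A door actor that toggles between closed and open when it receives an interaction request.
; On BeginPlay it stores its starting rotation as the closed pose and marks itself closed.
; Each Interact request flips the open flag and instantly sets the actor rotation, either back to the stored pose or to that pose combined with a -90 degree yaw, with no animated swing.
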(event `self.ReceiveBeginPlay`
  (set `self.InitialRotation` (`self.K2_GetActorRotation`))
  (set `self.DoorOpen` false))

(event `self.Interact.OnInteractRequset`
  (if (`self.DoorOpen`)
    (set `self.DoorOpen` false)
    (`self.K2_SetActorRotation` (`self.InitialRotation`))
    (else
      (set `self.DoorOpen` true)
      (`self.K2_SetActorRotation` (`KismetMathLibrary.ComposeRotators` (`KismetMathLibrary.MakeRotator` 0.0 0.0 -90.0) (`self.InitialRotation`))))))

(fn `UserConstructionScript`
  (`parent.UserConstructionScript`))