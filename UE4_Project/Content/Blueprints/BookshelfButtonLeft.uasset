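; Interactable button, by its name the left control for a bookshelf, that slides its linked actor along the X axis.
; On BeginPlay it caches the linked actor's starting location and sets a fixed X offset.
; An interact request plays a timeline only if the actor sits at start plus offset, adding the animated X value to that position.
; Otherwise it prints that the target cannot move further left.
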(event `self.ReceiveBeginPlay`
  (bind _returnvalue (`self.GetLinkedActor`))
  (set `self.LinkedInitialLocation` (`self.K2_GetActorLocation` _returnvalue))
  (set `self.Offset` (500.0 0.0 0.0)))

(event `self.InteractComponent.OnInteractRequest`
  (bind _returnvalue (`self.GetLinkedActor`))
  (if (== (`self.K2_GetActorLocation` _returnvalue) (+ (`self.LinkedInitialLocation`) (`self.Offset`)) :`ErrorTolerance` 0.0003)
    (bind (_direction _bookshelfanimation) (`Timeline|Timeline_0` :!via `PlayFromStart`)
      (:`Update`
        (bind _returnvalue_2 (`self.GetLinkedActor`))
        (`self.K2_SetActorLocation` _returnvalue_2 (+ (`KismetMathLibrary.MakeVector` _bookshelfanimation) (+ (`self.LinkedInitialLocation`) (`self.Offset`))) false false)))
    (else
      (`KismetSystemLibrary.PrintText` "Cannot move target more left." true false))))

(fn `UserConstructionScript`
  (`parent.UserConstructionScript`))