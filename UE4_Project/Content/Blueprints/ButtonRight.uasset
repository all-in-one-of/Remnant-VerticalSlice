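; Interactable button Blueprint that shifts its linked actor along the world X axis by a fixed step on each interaction.
; The Interact event adds RightOffset to the linked actor's current location, so repeated presses accumulate with no bounds check.
; A timeline then animates the button's Z offset from the resting location cached at BeginPlay.
; BeginPlay also stores the linked actor's initial location, though this graph never reads it.
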(event `self.ReceiveBeginPlay`
  (set `self.ButtonLocationDefault` (`self.K2_GetActorLocation`))
  (bind _returnvalue (`self.GetLinkedActor`))
  (set `self.InitialLocation` (`self.K2_GetActorLocation` _returnvalue))
  (set `self.RightOffset` (200.0 0.0 0.0)))

(event `self.Interact.OnInteractRequset`
  (bind _returnvalue (`self.GetLinkedActor`))
  (`self.K2_SetActorLocation` _returnvalue (+ (`self.K2_GetActorLocation` _returnvalue) (`self.RightOffset`)) false false)
  (bind (_direction _buttonz) (`Timeline|Timeline_0` :!via `PlayFromStart`)
    (:`Update`
      (`self.K2_SetActorLocation` (+ (`self.ButtonLocationDefault`) (`KismetMathLibrary.MakeVector` 0.0 0.0 _buttonz))))))

(fn `UserConstructionScript`
  (`parent.UserConstructionScript`))